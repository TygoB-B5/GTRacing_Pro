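; Player-controlled car Blueprint that forwards throttle/brake and steering axis input to its Throttle and Steer functions, whose logic is not in these graphs.
; BeginPlay spawns and plays an attached force feedback effect, and Tick scales its intensity by a Rumble value that is not set here.
; A temporary reset on right mouse button or gamepad bottom face button reloads the current level.
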(event `InputAxis|ThrottleBrake`
  (params (AxisValue :type "Float (single-precision)"))
  ;[1 1 1] Input
  (`self.Throttle` AxisValue))

(event `InputAxis|Steering`
  (params (AxisValue :type "Float (single-precision)"))
  ;[1 1 1] Input
  (`self.Steer` AxisValue))

(event `self.ReceiveBeginPlay`
  ;[1 1 1] Rumble Components
  (bind _returnvalue (`AddComponent|NODE_AddForceFeedbackComponent-0`))
  (bind _returnvalue_2 (`GameplayStatics.SpawnForceFeedbackAttached` "/Game/Misc/Rumble.Rumble" _returnvalue "None" (0.0 0.0 0.0) (struct) "KeepRelativeOffset" false true 1.0 0.0 null))
  (bind _output_get (set `self.Vibr` _returnvalue_2))
  (`ForceFeedbackComponent.Play` _output_get 0.0))

(event `self.ReceiveTick`
  (params (DeltaSeconds :type "Float (single-precision)"))
  ;[1 1 1] Rumble Components
  (`ForceFeedbackComponent.SetIntensityMultiplier` (`self.Vibr`) (`self.Rumble`)))

(event `Key|RightMouseButton`
  (params (Key :type "Key Structure"))
  ;[1 1 1] Temporary Reset
  (:`Pressed`
    (bind _returnvalue (`GameplayStatics.GetCurrentLevelName` true :!label _label))
    (`GameplayStatics.OpenLevel` (`KismetStringLibrary.Conv_StringToName` _returnvalue))))

(event `Key|Gamepad_FaceButton_Bottom`
  (params (Key :type "Key Structure"))
  ;[1 1 1] Temporary Reset
  (:`Pressed`
    (goto _label)))

(fn `UserConstructionScript`)