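; BP_SimpleCar is a bare-bones drivable car that takes player 0's input on BeginPlay.
; Steering input yaws the Car component and prints the scaled value, while ThrottleBrake input accumulates into an unclamped Speed.
; Tick teleports Car along Root's forward vector by Speed without sweep or delta-time scaling, so movement follows Root's heading rather than Car's.
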(event `self.ReceiveBeginPlay`
  (`self.EnableInput` (`GameplayStatics.GetPlayerController` 0)))

(event `InputAxis|Steering`
  (params (AxisValue :type "Float (single-precision)"))
  (bind _returnvalue (* AxisValue 0.5))
  (`KismetSystemLibrary.PrintString` (`KismetStringLibrary.Conv_DoubleToString` _returnvalue))
  (`SceneComponent.K2_AddWorldRotation` (`self.Car`) (`KismetMathLibrary.MakeRotator` 0.0 0.0 _returnvalue) false false))

(event `InputAxis|ThrottleBrake`
  (params (AxisValue :type "Float (single-precision)"))
  (set `self.Speed` (+ (`self.Speed`) AxisValue)))

(event `self.ReceiveTick`
  (params (DeltaSeconds :type "Float (single-precision)"))
  (`SceneComponent.K2_AddWorldOffset` (`self.Car`) (* (`SceneComponent.GetForwardVector` (`self.Root`)) (`self.Speed`)) false true))

(fn `UserConstructionScript`)